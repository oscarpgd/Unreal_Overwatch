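; Soldier: 76 character Blueprint that sets up the hero's health pool and sprint ability on top of a parent character class.
; BeginPlay initializes health, armor and shield values, then initializes SoldierSprintSkill with a Left Shift control label and adds it to the Skills list.
; The Skill_0 input action fires the sprint on Started and Triggered, and finishes it on Completed or Canceled.
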(event Input|EnhancedActionEvents|EnhancedInputActionSkill_0
  (params (ActionValue :type Boolean) (ElapsedSeconds :type Float%20%28double-precision%29) (TriggeredSeconds :type Float%20%28double-precision%29) (InputAction :type Input%20Action%20Object%20Reference :default "/Game/_Project/CommonSystems/Input/Skill_0.Skill_0"))
  (bind _soldier_sprint_skill (Variables|Default|GetSoldier_Sprint_Skill))
  (:Triggered
    (Default|Fire _soldier_sprint_skill :!label _label))
  (:Started
    (goto _label))
  (:Canceled
    (Default|Finish _soldier_sprint_skill :!label _label_2))
  (:Completed
    (goto _label_2)))

(event EventBeginPlay
  (bind _soldier_sprint_skill (Variables|Default|GetSoldier_Sprint_Skill))
  (|CallParentFunction)
  (Utilities|FlowControl|Sequence
    (:then_0
      (CallFunction|InitializeHealth (Utilities|Struct|MakeHealthData 125.0 125.0 5e+01 5e+01 5e+01 5e+01 0.0 false)))
    (:then_1
      (Default|Initialize _soldier_sprint_skill self "L SHIFT")
      (Utilities|Array|Add (Variables|Default|GetSkills) _soldier_sprint_skill))))

(fn ConstructionScript
  (|CallParentFunction))