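; Bob_BP is an AI-driven pawn that rams characters while running and tracks nearby Dummy actors.
; On a roughly head-on hit while BOB_AI_Controller reports IsRunning, it launches the struck Character forward and upward.
; The same hit calls the controller's OnCollide, even when the struck actor is not a Character.
; SphereRange overlap events add and remove Dummy actors in the Targets list.
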(event OnComponentBeginOverlap(SphereRange)
  (params (OverlappedComponent :type Primitive%20Component%20Object%20Reference) (OtherActor :type Actor%20Object%20Reference) (OtherComp :type Primitive%20Component%20Object%20Reference) (OtherBodyIndex :type Integer) (bFromSweep :type Boolean) (SweepResult :type Hit%20Result%20Structure%20%28by%20ref%29))
  (bind _asdummy (Utilities|Casting|CastToDummy OtherActor))
  (Utilities|Set|Add (Variables|Default|GetTargets) _asdummy))

(event OnComponentEndOverlap(SphereRange)
  (params (OverlappedComponent :type Primitive%20Component%20Object%20Reference) (OtherActor :type Actor%20Object%20Reference) (OtherComp :type Primitive%20Component%20Object%20Reference) (OtherBodyIndex :type Integer))
  (bind _asdummy (Utilities|Casting|CastToDummy OtherActor))
  (Utilities|Set|Remove (Variables|Default|GetTargets) _asdummy))

(event Collision|EventHit
  (params (MyComp :type Primitive%20Component%20Object%20Reference) (Other :type Actor%20Object%20Reference) (OtherComp :type Primitive%20Component%20Object%20Reference) (bSelfMoved :type Boolean) (HitLocation :type Vector :default "0, 0, 0") (HitNormal :type Vector :default "0, 0, 0") (NormalImpulse :type Vector :default "0, 0, 0") (Hit :type Hit%20Result%20Structure%20%28by%20ref%29))
  (if (and (< (Math|Vector|DotProduct HitNormal (Transformation|GetActorForwardVector)) -0.5) (Variables|/Game/_Project/Characters/AshenDash/BOB_AI_Controller.BOB_AI_Controller_C|GetIsRunning? (.AsBOB%20AI%20Controller (Utilities|Casting|CastToBOB_AI_Controller (Pawn|GetController)))))
    (Utilities|FlowControl|Sequence
      (:then_0
        (bind _ascharacter (Utilities|Casting|CastToCharacter Other))
        (Character|LaunchCharacter _ascharacter (+ (* (Transformation|GetActorForwardVector) 5e+02) "0.000000,0.000000,1000.000000") false false))
      (:then_1
        (Default|OnCollide (.AsBOB%20AI%20Controller (Utilities|Casting|CastToBOB_AI_Controller (Pawn|GetController))))))))

(fn ConstructionScript)